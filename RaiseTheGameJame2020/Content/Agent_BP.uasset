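; Agent Blueprint that exposes navigation requests and forwards them to its Agent_Controller.
; Events cover pathing to a position, testing whether a position is pathable, and moving to a random location, each casting the current controller first.
; The pathability result is saved in CanPathToLocation, and the random destination in PointerPosForPathfinding.
; It contains no pathfinding logic of its own, and its Tick and construction script are empty.
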(event EventBeginPlay)

(event Collision|EventActorBeginOverlap
  (params (OtherActor :type Actor%20Object%20Reference)))

(event EventTick
  (params (DeltaSeconds :type Float%20%28single-precision%29)))

(event EventPathfindtoLocation
  (params (position :type Vector :default "0, 0, 0"))
  (bind _asagent_controller (Utilities|Casting|CastToAgent_Controller (Pawn|GetController)))
  (Default|PathtoLocation _asagent_controller position))

(event EventIsLocationPathable
  (params (position :type Vector :default "0, 0, 0"))
  (bind _asagent_controller (Utilities|Casting|CastToAgent_Controller (Pawn|GetController)))
  (bind _pathable (Default|IsLocationPathable _asagent_controller position))
  (Variables|Default|SetCanPathToLocation _pathable))

(event EventGotoRandomLocation
  (bind _asagent_controller (Utilities|Casting|CastToAgent_Controller (Pawn|GetController)))
  (bind _locationtogoto (Default|GotoRandomLocation _asagent_controller))
  (Variables|Default|SetPointerPosForPathfinding _locationtogoto))

(fn ConstructionScript)